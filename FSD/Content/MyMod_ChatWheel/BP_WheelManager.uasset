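; Manager actor for the chat wheel mod that shows the wheel while a configurable key is held.
; The key press lazily creates the wheel widget, locks look input and centres the mouse; release or abort restores the saved cursor and input state.
; BeginPlay loads key and messages from a SaveGame or applies defaults, while update functions save changes asynchronously.
; Dispatchers announce wheel opening, closing and completed saves.
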(event `Execute_AsyncSave`
  (`AsyncActionHandleSaveGame.AsyncSaveGameToSlot` (`self.Ref_SaveGameObject`) (`self.SaveSlotName`)
    (:`Completed`
      (`self.OnModDataUpdated`))))

(event `Key|AnyKey` :consume false
  (params (Key :type "Key Structure"))
  (bind _localplayer (`/Game/DRGLib/DRGFunctions/LIB_F_DRG.GetLocalPlayerController`))
  (bind _localplayer_2 (`/Game/DRGLib/DRGFunctions/LIB_F_DRG.GetLocalPlayerController`))
  (bind _localplayer_3 (`/Game/DRGLib/DRGFunctions/LIB_F_DRG.GetLocalPlayerController`))
  (bind _returnvalue (== Key (`self.ActiveWheelKey`)))
  (bind (_x _y) (`KismetMathLibrary.BreakVector2D` (/ (`WidgetLayoutLibrary.GetViewportSize`) 2.0)))
  (:`Pressed`
    (if _returnvalue
      (`/Engine/EditorBlueprintResources/StandardMacros.IsValid` (`self.Ref_ChatWheel_UI`)
        (:`Is Valid`
          _)
        (:`Is Not Valid`
          ;[1 1 1] 绘制UI
          (bind _returnvalue_2 (`|CreateWidget` "/Game/MyMod_ChatWheel/Widgets/WBP_ChatWheel_UI.WBP_ChatWheel_UI_C" (`/Game/DRGLib/DRGFunctions/LIB_F_DRG.GetLocalPlayerController`)))
          (set `self.Ref_ChatWheel_UI` _returnvalue_2)
          (`UserWidget.AddToPlayerScreen` _returnvalue_2 1)))
      (`self.OnWheelOpened`)
      (set `self.bWasMouseVisible` (`PlayerController.bShowMouseCursor` _localplayer_2))
      (set `self.bWasLookIgnored` (`Controller.IsLookInputIgnored` _localplayer_2))
      (set `self.bIsWheelOpen` true)
      (`Controller.SetIgnoreLookInput` (`/Game/DRGLib/DRGFunctions/LIB_F_DRG.GetLocalPlayerController`) true)
      ;[1 1 1] 鼠标回正
      (`PlayerController.SetMouseLocation` _localplayer (`KismetMathLibrary.FTrunc` _x) (`KismetMathLibrary.FTrunc` _y))
      (`WidgetBlueprintLibrary.SetInputMode_GameAndUIEx` _localplayer (`self.Ref_WheelUI`))))
  (:`Released`
    (if _returnvalue
      (`self.OnWheelClosed`)
      (set `self.bIsWheelOpen` false)
      (set `PlayerController.bShowMouseCursor` (`self.bWasMouseVisible`) _localplayer_3)
      (`Controller.SetIgnoreLookInput` _localplayer_3 (`self.bWasLookIgnored`))
      (if (`self.bWasMouseVisible`)
        (`WidgetBlueprintLibrary.SetInputMode_GameAndUIEx` null null)
        (else
          (`WidgetBlueprintLibrary.SetInputMode_GameOnly` _localplayer_3))))))

(event `self.ReceiveBeginPlay`
  ;[1 1 1] 读取保存的设置
  (bind _returnvalue (`GameplayStatics.LoadGameFromSlot` (`self.SaveSlotName`)))
  (bind _assg_chat_wheel_config (cast `/Game/MyMod_ChatWheel/Save/SG_ChatWheel_Config` _returnvalue)
    (:`then`
      (set `self.Ref_SaveGameObject` _assg_chat_wheel_config)
      (set `self.ActiveWheelKey` (`/Game/MyMod_ChatWheel/Save/SG_ChatWheel_Config.ActiveWheelKey` _assg_chat_wheel_config))
      (set `self.CustomMessages` (`/Game/MyMod_ChatWheel/Save/SG_ChatWheel_Config.CustomMessages` _assg_chat_wheel_config)))
    (:`CastFailed`
      (bind _returnvalue_2 (`GameplayStatics.CreateSaveGameObject` "/Game/MyMod_ChatWheel/Save/SG_ChatWheel_Config.SG_ChatWheel_Config_C"))
      (bind _output_get (set `self.Ref_SaveGameObject` _returnvalue_2))
      ;;[1 1 1] 默认设置
      (set `self.CustomMessages` (`self.DefaultMessages`))
      (set `self.ActiveWheelKey` "T")
      (`GameplayStatics.SaveGameToSlot` _output_get (`self.SaveSlotName`))))
  (`self.EnableInput` (`/Game/DRGLib/DRGFunctions/LIB_F_DRG.GetLocalPlayerController`)))

(fn `UpdateKeyOnly`
  (params (NewKey :type "Key Structure" :default "None"))
  (bind _ref_savegameobject (`self.Ref_SaveGameObject`))
  (set `self.ActiveWheelKey` NewKey)
  (`/Engine/EditorBlueprintResources/StandardMacros.IsValid` _ref_savegameobject
    (:`Is Valid`
      (set `/Game/MyMod_ChatWheel/Save/SG_ChatWheel_Config.ActiveWheelKey` NewKey _ref_savegameobject))
    (:`Is Not Valid`
      (bind _returnvalue (`GameplayStatics.CreateSaveGameObject` "/Game/MyMod_ChatWheel/Save/SG_ChatWheel_Config.SG_ChatWheel_Config_C"))
      (set `self.Ref_SaveGameObject` _returnvalue)))
  (`self.Execute_AsyncSave`))

(fn `UpdateMessagesOnly`
  (params (NewMessages :type "Array of Text"))
  (bind _ref_savegameobject (`self.Ref_SaveGameObject`))
  (set `self.CustomMessages` NewMessages)
  (`/Engine/EditorBlueprintResources/StandardMacros.IsValid` _ref_savegameobject
    (:`Is Valid`
      (set `/Game/MyMod_ChatWheel/Save/SG_ChatWheel_Config.CustomMessages` NewMessages _ref_savegameobject))
    (:`Is Not Valid`
      (bind _returnvalue (`GameplayStatics.CreateSaveGameObject` "/Game/MyMod_ChatWheel/Save/SG_ChatWheel_Config.SG_ChatWheel_Config_C"))
      (set `self.Ref_SaveGameObject` _returnvalue)))
  (`self.Execute_AsyncSave`))

(fn `UpdateModSettings`
  (params (Newkey :type "Key Structure" :default "None") (NewMessages :type "Array of Text"))
  (set `self.ActiveWheelKey` Newkey)
  (set `self.CustomMessages` NewMessages)
  (`/Engine/EditorBlueprintResources/StandardMacros.IsValid` (`self.Ref_SaveGameObject`)
    (:`Is Valid`
      _)
    (:`Is Not Valid`
      (bind _returnvalue (`GameplayStatics.CreateSaveGameObject` "/Game/MyMod_ChatWheel/Save/SG_ChatWheel_Config.SG_ChatWheel_Config_C"))
      (bind _output_get (set `self.Ref_SaveGameObject` _returnvalue))))
  (set `/Game/MyMod_ChatWheel/Save/SG_ChatWheel_Config.CustomMessages` NewMessages _output_get)
  (set `/Game/MyMod_ChatWheel/Save/SG_ChatWheel_Config.ActiveWheelKey` Newkey _output_get)
  (`self.Execute_AsyncSave`)
  (bind _ref_wheelui (`self.Ref_WheelUI`)
    (:`then`
      (`/Game/MyMod_ChatWheel/Widgets/WBP_ChatWheel_UI.RefreshWheelTexts` _ref_wheelui))
    (:`else`)))

(fn `UserConstructionScript`)

(fn `WheelAbort`
  (bind _localplayer (`/Game/DRGLib/DRGFunctions/LIB_F_DRG.GetLocalPlayerController`))
  (set `self.CurrentSelectedIndex` -1)
  (`self.OnWheelClosed`)
  (set `PlayerController.bShowMouseCursor` (`self.bWasMouseVisible`) _localplayer)
  (`Controller.SetIgnoreLookInput` _localplayer (`self.bWasLookIgnored`))
  (if (`self.bWasMouseVisible`)
    (`WidgetBlueprintLibrary.SetInputMode_GameAndUIEx` null null)
    (else
      (`WidgetBlueprintLibrary.SetInputMode_GameOnly` _localplayer))))